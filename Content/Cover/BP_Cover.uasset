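; BP_Cover is a destructible cover actor that the player can take cover behind and that respawns after being destroyed.
; Overlaps on its collision component toggle a can-enter-cover flag, and damage lowers clamped health shown on a widget health bar.
; At zero health it forces BP_Player out of cover, cancels reloading, and hides with collision off.
; After a short delay it restores health, visibility, collision and the bar.
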(event `self.ReceiveBeginPlay`
  (set `self.CoverHealth` (`self.MaxCoverHealth`)))

(event `self.CoverCollision.OnComponentBeginOverlap`
  (params (OverlappedComponent :type "PrimitiveComponent Object Reference") (OtherActor :type "Actor Object Reference") (OtherComp :type "PrimitiveComponent Object Reference") (OtherBodyIndex :type Integer) (bFromSweep :type Boolean) (SweepResult :type "HitResult Structure (by ref)"))
  (set `self.CanInCover` true))

(event `self.CoverCollision.OnComponentEndOverlap`
  (params (OverlappedComponent :type "PrimitiveComponent Object Reference") (OtherActor :type "Actor Object Reference") (OtherComp :type "PrimitiveComponent Object Reference") (OtherBodyIndex :type Integer))
  (set `self.CanInCover` false))

(event `self.ReceiveAnyDamage`
  (params (Damage :type "Float (single-precision)") (DamageType :type "DamageType Object Reference") (InstigatedBy :type "Controller Object Reference") (DamageCauser :type "Actor Object Reference"))
  (set `self.CoverHealth` (`KismetMathLibrary.FClamp` (- (`self.CoverHealth`) Damage) 0.0 (`self.MaxCoverHealth`)))
  (bind _aswbp_cover_health_bar (cast `/Game/Cover/WBP_CoverHealthBar` (`WidgetComponent.GetUserWidgetObject` (`self.HealthBarWidget`))))
  (`/Game/Cover/WBP_CoverHealthBar.UpdateHealthBar` _aswbp_cover_health_bar (/ (`self.CoverHealth`) (`self.MaxCoverHealth`)))
  (if (<= (`self.CoverHealth`) 0.0)
    (`self.DestroyedCover`)
    (bind _returnvalue (`GameplayStatics.GetActorOfClass` "/Game/Characters/BP_Player.BP_Player_C"))
    (`Character.StopAnimMontage` _returnvalue "/Game/Characters/Mannequins/Anims/Rifle/AM_Reload.AM_Reload")))

(event `DestroyedCover`
  (bind _returnvalue (`GameplayStatics.GetActorOfClass` "/Game/Characters/BP_Player.BP_Player_C"))
  (if (`/Game/Characters/BP_Player.IsInCover` _returnvalue)
    (`/Game/Characters/BP_Player.OutCover` _returnvalue)
    (set `/Game/Characters/BP_Player.IsReloading` false _returnvalue))
  (`self.SetActorHiddenInGame` true)
  (`PrimitiveComponent.SetCollisionEnabled` (`self.Cover`) "NoCollision")
  (`PrimitiveComponent.SetCollisionEnabled` (`self.CoverCollision`) "NoCollision")
  (`KismetSystemLibrary.Delay` 5.0)
  (`self.SpawnCover`))

(event `SpawnCover`
  (set `self.CoverHealth` (`self.MaxCoverHealth`))
  (`self.SetActorHiddenInGame` false)
  (`PrimitiveComponent.SetCollisionEnabled` (`self.Cover`) "QueryAndPhysics")
  (`PrimitiveComponent.SetCollisionEnabled` (`self.CoverCollision`) "QueryOnly")
  (bind _aswbp_cover_health_bar (cast `/Game/Cover/WBP_CoverHealthBar` (`WidgetComponent.GetUserWidgetObject` (`self.HealthBarWidget`))))
  (`/Game/Cover/WBP_CoverHealthBar.UpdateHealthBar` _aswbp_cover_health_bar (/ (`self.CoverHealth`) (`self.MaxCoverHealth`))))

(fn `UserConstructionScript`)