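; Enemy pawn that moves to a randomly chosen BP_MovePoint, then turns to face the player and shoots.
; On arrival it yaws toward the player each tick and a looping timer fires three-shot bursts of BP_EnemyBullet.
; Bullets spawn at a fixed world-forward offset, with no rotation passed.
; TakeDamage clamps health and updates the health bar widget, with no death handling.
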(event `self.ReceiveBeginPlay`
  (set `self.EnemyHealth` (`self.MaxEnemyHealth`))
  (bind _outactors (`GameplayStatics.GetAllActorsOfClass` "/Game/Enemy/BP_MovePoint.BP_MovePoint_C"))
  (bind _output_get (set `self.MovePoint` (`|GetArrayItem` _outactors (`KismetMathLibrary.RandomIntegerInRange` 0 (- (`KismetArrayLibrary.Array_Length` _outactors) 1)))))
  (`|AIMoveTo` self (`self.K2_GetActorLocation` _output_get) null
    (:`then`
      (bind _asbp_player (cast `/Game/Characters/BP_Player` (`GameplayStatics.GetPlayerCharacter` 0)))
      (set `self.Player` _asbp_player))
    (:`OnSuccess`
      (set `self.IsArrived` true)
      (set `self.CanAttack` true)
      (`KismetSystemLibrary.K2_SetTimerDelegate` (delegate `Attack`) 3.3 true))))

(event `self.ReceiveTick`
  (params (DeltaSeconds :type "Float (single-precision)"))
  (if (`self.IsArrived`)
    (`self.K2_SetActorRotation` (`KismetMathLibrary.MakeRotator` 0.0 0.0 (.yaw (`KismetMathLibrary.FindLookAtRotation` (`self.K2_GetActorLocation`) (`self.K2_GetActorLocation` (`self.Player`))))))))

(event `Attack`
  (if (`self.CanAttack`)
    (`self.Fire`)
    (`KismetSystemLibrary.Delay` 0.15)
    (`self.Fire`)
    (`KismetSystemLibrary.Delay` 0.15)
    (`self.Fire`)))

(fn `Fire`
  (`|SpawnActorFromClass` "/Game/Enemy/BP_EnemyBullet.BP_EnemyBullet_C" (`KismetMathLibrary.Conv_VectorToTransform` (+ (`self.K2_GetActorLocation`) (* (`KismetMathLibrary.Vector_Forward`) 100))) "Undefined" "MultiplyWithRoot" null null))

(fn `TakeDamage`
  (params (DamgeAmount :type "Float (double-precision)"))
  (set `self.EnemyHealth` (`KismetMathLibrary.FClamp` (- (`self.EnemyHealth`) DamgeAmount) 0.0 (`self.MaxEnemyHealth`)))
  (bind _aswbp_enemy_health_bar (cast `/Game/Enemy/WBP_EnemyHealthBar` (`WidgetComponent.GetUserWidgetObject` (`self.HealthBarWidget`))))
  (`/Game/Enemy/WBP_EnemyHealthBar.UpdateHealthBar` _aswbp_enemy_health_bar (/ (`self.EnemyHealth`) (`self.MaxEnemyHealth`))))

(fn `UserConstructionScript`)