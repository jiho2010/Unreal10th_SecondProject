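; BP_SpawnManager is an enemy spawn manager that spawns a drone at a move point on BeginPlay.
; SpawnDrone spawns the drone class at a valid SelectedMovePoint, hands it that point, then marks the point occupied and clears its CurrentDrone.
; FindEmptyMovePoint picks and reserves a random unoccupied point from MovePointArray, but nothing in this graph calls it, so spawning relies on SelectedMovePoint already being set.
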(event `self.ReceiveBeginPlay`
  (`self.SpawnDrone`))

(fn `FindEmptyMovePoint`
  (`KismetArrayLibrary.Array_Clear` (`self.AvailableMovePoints`))
  (for _array_element (`self.MovePointArray`)
    (if (not (`/Game/Enemy/BP_MovePoint.IsOccupied` _array_element))
      (`KismetArrayLibrary.Array_Add` (`self.AvailableMovePoints`) _array_element)))
  (if (> (`KismetArrayLibrary.Array_Length` (`self.AvailableMovePoints`)) 0)
    (bind _output_get (set `self.SelectedMovePoint` (`KismetArrayLibrary.Array_Random` (`self.AvailableMovePoints`))))
    (set `/Game/Enemy/BP_MovePoint.IsOccupied` true _output_get)))

(fn `SpawnDrone`
  (`/Engine/EditorBlueprintResources/StandardMacros.IsValid` (`self.SelectedMovePoint`)
    (:`Is Valid`
      (bind _returnvalue (`|SpawnActorFromClass` (`self.DroneClass`) (`self.GetTransform` (`self.SelectedMovePoint`)) "Undefined" "MultiplyWithRoot" null null))
      (bind _output_get (set `/Game/Enemy/BP_Enemy.MovePoint` (`self.SelectedMovePoint`) _returnvalue))
      (set `/Game/Enemy/BP_MovePoint.CurrentDrone` null _output_get)
      (set `/Game/Enemy/BP_MovePoint.IsOccupied` true _output_get))))

(fn `UserConstructionScript`)