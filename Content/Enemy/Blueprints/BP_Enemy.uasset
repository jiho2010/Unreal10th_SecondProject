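; BP_Enemy is a shooting enemy that moves to its assigned MovePoint, then faces the player and fires at them.
; After a short delay it uses AIMoveTo; on arrival, Tick tracks the player and a looping timer fires three-shot bursts from the Muzzle socket.
; Damage updates its health bar widget.
; Death frees the MovePoint, asks SpawnManager for the next enemy, destroys the actor and notifies the player's MainTitle.
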(event `self.ReceiveBeginPlay`
  (set `self.EnemyHealth` (`self.MaxEnemyHealth`))
  (`KismetSystemLibrary.Delay` 1.5)
  (`|AIMoveTo` self (`self.K2_GetActorLocation` (`self.MovePoint`)) null
    (:`then`
      (bind _asbp_player (cast `/Game/Characters/Blueprints/BP_Player` (`GameplayStatics.GetPlayerCharacter` 0)))
      (set `self.Player` _asbp_player))
    (:`OnSuccess`
      (set `self.IsArrived` true)
      (set `self.CanAttack` true)
      (`KismetSystemLibrary.K2_SetTimerDelegate` (delegate `Attack`) 3.0 true))))

(event `self.ReceiveTick`
  (params (DeltaSeconds :type "Float (single-precision)"))
  (if (`self.IsArrived`)
    (`self.K2_SetActorRotation` (`KismetMathLibrary.MakeRotator` (.roll (`KismetMathLibrary.FindLookAtRotation` (`self.K2_GetActorLocation`) (`self.K2_GetActorLocation` (`self.Player`)))) (.pitch (`KismetMathLibrary.FindLookAtRotation` (`self.K2_GetActorLocation`) (`self.K2_GetActorLocation` (`self.Player`)))) (.yaw (`KismetMathLibrary.FindLookAtRotation` (`self.K2_GetActorLocation`) (`self.K2_GetActorLocation` (`self.Player`))))))))

(event `Attack`
  (if (`self.CanAttack`)
    (`self.Fire`)
    (`KismetSystemLibrary.Delay` 0.2)
    (`self.Fire`)
    (`KismetSystemLibrary.Delay` 0.2)
    (`self.Fire`)))

(event `self.ReceiveAnyDamage`
  (params (Damage :type "Float (single-precision)") (DamageType :type "DamageType Object Reference") (InstigatedBy :type "Controller Object Reference") (DamageCauser :type "Actor Object Reference"))
  (if (not (`self.IsDead`))
    (set `self.EnemyHealth` (`KismetMathLibrary.FClamp` (- (`self.EnemyHealth`) Damage) 0.0 (`self.MaxEnemyHealth`)))
    (bind _aswbp_enemy_health_bar (cast `/Game/Enemy/Blueprints/WBP_EnemyHealthBar` (`WidgetComponent.GetUserWidgetObject` (`self.HealthBarWidget`))))
    (`/Game/Enemy/Blueprints/WBP_EnemyHealthBar.UpdateHealthBar` _aswbp_enemy_health_bar (/ (`self.EnemyHealth`) (`self.MaxEnemyHealth`)))
    (if (<= (`self.EnemyHealth`) 0.0)
      (`self.Die`))))

(event `Die`
  (set `/Game/Enemy/Blueprints/BP_MovePoint.IsOccupied` false (`self.MovePoint`))
  (set `self.IsDead` true)
  (`/Game/Enemy/Blueprints/BP_SpawnManager.SpawnNextEnemy` (`self.SpawnManager`))
  (`self.K2_DestroyActor`)
  (`/Game/Characters/Blueprints/WBP_PlayerUI.SetDied` (`/Game/Characters/Blueprints/BP_Player.MainTitle` (`self.Player`))))

(fn `Fire`
  (`|SpawnActorFromClass` "/Game/Enemy/Blueprints/BP_EnemyBullet.BP_EnemyBullet_C" (`SceneComponent.GetSocketTransform` (`self.Mesh`) "Muzzle" "RTS_World") "Undefined" "MultiplyWithRoot" null null))

(fn `UserConstructionScript`)